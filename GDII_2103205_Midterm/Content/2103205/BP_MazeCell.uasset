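; A maze cell actor that builds its floor and optional walls and recolors its spotlight from player gate events.
; The construction script scales the floor from GridSize and adds a static mesh for each enabled wall flag, deriving thickness from cell size and converting dimensions through SizeToCubeScale.
; On BeginPlay it binds to the third-person character's MazeGate event, applying that character's LightColor whenever the event reports not inside.
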(event Custom|MazeGate_Event
  (params (IsInside :type Boolean))
  (bind _spotlight (Variables|Default|GetSpotLight))
  (if (not IsInside)
    (Utilities|IsValid _spotlight
      (:Is%20Valid
        (Rendering|Components|Light|SetLightColor _spotlight (Variables|/Game/2103205/Blueprints/BP_ThirdPersonCharacter.BP_ThirdPersonCharacter_C|GetLightColor (Variables|Default|GetAs%20BP%20Third%20Person%20Character)) true)))))

(event EventBeginPlay
  (bind _output_get (Variables|Default|SetAs%20BP%20Third%20Person%20Character (.AsBP%20Third%20Person%20Character (Utilities|Casting|CastToBP_ThirdPersonCharacter (Game|Player|GetPlayerPawn 0)))))
  (EventDispatchers|BindEventtoMazeGate _output_get (delegate Custom|MazeGate_Event)))

(fn ConstructionScript
  (bind _gridsize (Variables|Default|GetGridSize))
  (bind _wallheight (Variables|Default|GetWallHeight))
  (LocalVariables|SetWall%20Lenght _gridsize)
  (LocalVariables|SetWall%20Thichkness (* _gridsize 0.1))
  (Transformation|SetRelativeScale3D (Variables|Default|GetFloor) (Utilities|SizetoCubeScale (Math|Vector|MakeVector (LocalVariables|GetWall%20Lenght) (LocalVariables|GetWall%20Lenght) (LocalVariables|GetWall%20Thichkness))))
  (Utilities|FlowControl|Sequence
    (:then_0
      (if (Variables|Default|GetWestWall)
        (AddComponent|AddStaticMeshComponent false (Math|Transform|MakeTransform (Math|Vector|MakeVector 0.0 0.0 0.0) "0, 0, 0" (Utilities|SizetoCubeScale (Math|Vector|MakeVector (LocalVariables|GetWall%20Lenght) (LocalVariables|GetWall%20Thichkness) _wallheight))))))
    (:then_1
      (if (Variables|Default|GetSouthWall)
        (AddComponent|AddStaticMeshComponent false (Math|Transform|MakeTransform (Math|Vector|MakeVector 0.0 0.0 0.0) "0, 0, 0" (Utilities|SizetoCubeScale (Math|Vector|MakeVector (LocalVariables|GetWall%20Thichkness) (LocalVariables|GetWall%20Lenght) _wallheight))))))
    (:then_2
      (if (Variables|Default|GetNorthWall)
        (AddComponent|AddStaticMeshComponent false (Math|Transform|MakeTransform (Math|Vector|MakeVector (- (LocalVariables|GetWall%20Lenght) (LocalVariables|GetWall%20Thichkness)) 0.0 0.0) "0, 0, 0" (Utilities|SizetoCubeScale (Math|Vector|MakeVector (LocalVariables|GetWall%20Thichkness) (LocalVariables|GetWall%20Lenght) _wallheight))))))
    (:then_3
      (if (Variables|Default|GetEastWall)
        (AddComponent|AddStaticMeshComponent false (Math|Transform|MakeTransform (Math|Vector|MakeVector 0.0 (- (LocalVariables|GetWall%20Lenght) (LocalVariables|GetWall%20Thichkness)) 0.0) "0, 0, 0" (Utilities|SizetoCubeScale (Math|Vector|MakeVector (LocalVariables|GetWall%20Lenght) (LocalVariables|GetWall%20Thichkness) _wallheight))))))))