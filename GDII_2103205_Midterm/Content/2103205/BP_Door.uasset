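; BP_Door is a locked door that slides open on interaction when the game mode's Keys value equals the door's KeyNumber.
; BeginPlay caches Main_GameMode for that check, and a mismatch prints a wrong-key message.
; Despite its name, the Door_Rotate timeline moves the door mesh's relative location between start and finish vectors.
; The construction script applies a configurable material to the mesh.
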(event EventBeginPlay
  (Variables|Default|SetAs%20Main%20Game%20Mode (.AsMain%20Game%20Mode (Utilities|Casting|CastToMain_GameMode (Game|GetGameMode)))))

(event EventInteract
  (if (== (Variables|/Game/2103205/Main_GameMode.Main_GameMode_C|GetKeys (Variables|Default|GetAs%20Main%20Game%20Mode)) (Variables|Default|GetKey%20Number))
    (bind _newtrack_0 (Timeline|Door_Rotate Play)
      (:Update
        (Transformation|SetRelativeLocation (Variables|Default|GetSM%20Door) (Math|Vector|Lerp(Vector) (Variables|Default|GetStart%20Location) (Variables|Default|GetFinish%20Location) _newtrack_0) false false)))
    (else
      (Development|PrintString "You don't have the correct key."))))

(fn ConstructionScript
  (Rendering|Material|SetMaterial (Variables|Default|GetSM%20Door) 0 (Variables|Default|GetMaterial)))