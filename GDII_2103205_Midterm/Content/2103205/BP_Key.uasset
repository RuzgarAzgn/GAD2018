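; BP_Key is a key pickup actor that records its key number on the game mode when interacted with.
; It caches Main_GameMode at BeginPlay, and Interact overwrites its Keys value with KeyNumber, prints the acquired key's name from Names, then destroys the actor.
; The construction script applies the Material variable to the Key component, so each placed key can look different.
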(event EventBeginPlay
  (Variables|Default|SetAs%20Main%20Game%20Mode (.AsMain%20Game%20Mode (Utilities|Casting|CastToMain_GameMode (Game|GetGameMode)))))

(event EventInteract
  (bind _output_get (Variables|/Game/2103205/Main_GameMode.Main_GameMode_C|SetKeys (Variables|Default|GetAs%20Main%20Game%20Mode) (Variables|Default|GetKey%20Number)))
  (Development|PrintString (Utilities|String|Append "Key " (Utilities|Array|Get(acopy) (Variables|Default|GetNames) _output_get) " Acquired"))
  (Actor|DestroyActor))

(fn ConstructionScript
  (Rendering|Material|SetMaterial (Variables|Default|GetKey) 0 (Variables|Default|GetMaterial)))